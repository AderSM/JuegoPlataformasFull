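; BP_BulletEnemy is an enemy projectile that damages the player on contact.
; Each tick it moves itself along its forward vector at a fixed speed, without sweeping or a movement component.
; An overlap with an actor tagged Player applies damage and destroys the bullet, while a timer started at BeginPlay destroys it after a short lifetime.
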(event Custom|Destroy
  (Actor|DestroyActor))

(event EventBeginPlay
  (Utilities|Time|SetTimerbyEvent (delegate Custom|Destroy) 2.5))

(event Collision|EventActorBeginOverlap
  (params (OtherActor :type Actor%20Object%20Reference))
  (if (Utilities|Array|ContainsItem (Variables|/Script/Engine.Actor|GetTags OtherActor) "Player")
    (Game|Damage|ApplyDamage OtherActor 2e+01 0 0)
    (Actor|DestroyActor)))

(event EventTick
  (params (DeltaSeconds :type Float%20%28single-precision%29))
  (Transformation|SetActorLocation (+ (Transformation|GetActorLocation) (* (* DeltaSeconds 1e+03) (Transformation|GetActorForwardVector))) false false))

(fn ConstructionScript)